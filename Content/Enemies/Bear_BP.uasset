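; Bear enemy that wanders around its spawn point, chases the player on sight, and can kill or be killed on contact.
; Patrol picks random destinations within a movement radius by line tracing down from high altitude, pausing after each successful move.
; PawnSensing starts a chase toward the player, with a retriggerable delay that resumes patrol.
; Player overlap with one box sets Dead and plays the death animation; the other destroys the player while the bear lives.
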(event OnSeePawn(PawnSensing)
  (params (Pawn :type Pawn%20Object%20Reference))
  (if (not (Variables|Default|GetDead))
    (bind _asthird_person_character (Utilities|Casting|CastToThirdPersonCharacter Pawn)
      (:then
        (AI|AIMoveTo self "0, 0, 0" _asthird_person_character 7e+01 false
          (:then
            (Utilities|FlowControl|RetriggerableDelay 5.0)
            (CallFunction|Patrullar))))
      (:CastFailed
        (Development|PrintString "FAILED sensing")))))

(event OnComponentBeginOverlap(KillCollisionBox)
  (params (OverlappedComponent :type Primitive%20Component%20Object%20Reference) (OtherActor :type Actor%20Object%20Reference) (OtherComp :type Primitive%20Component%20Object%20Reference) (OtherBodyIndex :type Integer) (bFromSweep :type Boolean) (SweepResult :type Hit%20Result%20Structure%20%28by%20ref%29))
  (bind _asthird_person_character (Utilities|Casting|CastToThirdPersonCharacter OtherActor))
  (if (not (Variables|Default|GetDead))
    (Actor|DestroyActor _asthird_person_character)))

(event OnComponentBeginOverlap(DeadCollisionBox)
  (params (OverlappedComponent :type Primitive%20Component%20Object%20Reference) (OtherActor :type Actor%20Object%20Reference) (OtherComp :type Primitive%20Component%20Object%20Reference) (OtherBodyIndex :type Integer) (bFromSweep :type Boolean) (SweepResult :type Hit%20Result%20Structure%20%28by%20ref%29))
  (Utilities|Casting|CastToThirdPersonCharacter OtherActor)
  (Variables|Default|SetDead true)
  (Components|Animation|PlayAnimation (Variables|Character|GetMesh) "/Game/InfinityBladeAdversaries/Enemy/Enemy_Bear/Enemy_Bear_Animations/ExoGame_Bears_Attack_Death.ExoGame_Bears_Attack_Death" false))

(event Custom|Patrullar
  (bind _radiodemovimiento (Variables|Default|GetRadioDeMovimiento))
  (bind _radiodemovimiento_2 (Variables|Default|GetRadioDeMovimiento))
  (bind _ubicacioninicial (Variables|Default|GetUbicacionInicial))
  (bind _radiodemovimiento_3 (Variables|Default|GetRadioDeMovimiento))
  (bind _radiodemovimiento_4 (Variables|Default|GetRadioDeMovimiento))
  (bind _returnvalue (* _radiodemovimiento_4 -1.0))
  (bind _returnvalue_2 (* _radiodemovimiento -1.0))
  (bind _returnvalue_3 (Math|Random|RandomFloatinRange _returnvalue _radiodemovimiento_2))
  (bind _returnvalue_4 (Math|Random|RandomFloatinRange _returnvalue_2 _radiodemovimiento_3))
  (bind _returnvalue_5 (+ _returnvalue_4 (.x _ubicacioninicial)))
  (bind _returnvalue_6 (+ _returnvalue_3 (.y _ubicacioninicial)))
  (if (not (Variables|Default|GetDead)) :!label _label
    (bind _outhit (Collision|LineTraceByChannel (Math|Vector|MakeVector _returnvalue_5 _returnvalue_6 2.5e+04) (Math|Vector|MakeVector _returnvalue_5 _returnvalue_6 0.0) "TraceTypeQuery1" false 0 "None" true "(R=1.000000,G=0.000000,B=0.000000,A=1.000000)" "(R=0.000000,G=1.000000,B=0.000000,A=1.000000)" 5.0))
    (AI|AIMoveTo self (.ImpactPoint (Collision|BreakHitResult _outhit)) 0 5.0 false
      (:OnSuccess
        (Utilities|FlowControl|Delay 5.0)
        (goto _label)))))

(event EventBeginPlay
  (Variables|Default|SetUbicacionInicial (Transformation|GetActorLocation))
  (CallFunction|Patrullar))

(event Collision|EventActorBeginOverlap
  (params (OtherActor :type Actor%20Object%20Reference)))

(event EventTick
  (params (DeltaSeconds :type Float%20%28single-precision%29)))

(fn ConstructionScript)