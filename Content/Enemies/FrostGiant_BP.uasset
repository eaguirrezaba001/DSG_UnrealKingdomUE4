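; Frost Giant enemy Blueprint that plays a scripted animation sequence when PawnSensing spots the ThirdPersonCharacter.
; After timed delays it plays an aggro animation, then a trap magic animation, then settles into a looping stunned idle.
; Animations play directly on the mesh, chained by Delay nodes, with a Retriggerable Delay before the idle that restarts whenever execution reaches it again.
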(event OnSeePawn(PawnSensing)
  (params (Pawn :type Pawn%20Object%20Reference))
  (bind _mesh (Variables|Character|GetMesh))
  (Utilities|Casting|CastToThirdPersonCharacter Pawn)
  (Utilities|FlowControl|Delay 3.2)
  (Components|Animation|PlayAnimation _mesh "/Game/InfinityBladeAdversaries/Enemy/Enemy_Frost_Giant/Enemy_Frost_Giant_All_Animation/ExoGame_FrostGiant_Aggro.ExoGame_FrostGiant_Aggro" false)
  (Utilities|FlowControl|Delay 2.9)
  (Components|Animation|PlayAnimation _mesh "/Game/InfinityBladeAdversaries/Enemy/Enemy_Frost_Giant/Enemy_Frost_Giant_All_Animation/ExoGame_FrostGiant_Trap_Magic.ExoGame_FrostGiant_Trap_Magic" false)
  (Utilities|FlowControl|Delay 3.2)
  (Utilities|FlowControl|RetriggerableDelay 9.5)
  (Components|Animation|PlayAnimation (Variables|Character|GetMesh) "/Game/InfinityBladeAdversaries/Enemy/Enemy_Frost_Giant/Enemy_Frost_Giant_All_Animation/ExoGame_FrostGiant_React_Stunned_Idle.ExoGame_FrostGiant_React_Stunned_Idle" true))

(event EventBeginPlay)

(event Collision|EventActorBeginOverlap
  (params (OtherActor :type Actor%20Object%20Reference)))

(event EventTick
  (params (DeltaSeconds :type Float%20%28single-precision%29)))

(fn ConstructionScript)